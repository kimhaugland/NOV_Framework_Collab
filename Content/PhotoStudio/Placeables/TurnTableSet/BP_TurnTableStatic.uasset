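; Photo studio turntable stage placeable, built from center plate, outer plate, wall and ramp meshes.
; The construction script picks the outer floor mesh from a floor-type map or a custom override, then applies the selected materials, with wall and ramp sharing one.
; A separate AttachCarActor function makes a car actor movable and snaps it to the center plate, keeping relative scale; no graph here calls it.
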(fn `AttachCarActor`
  (bind (_x _y) (`KismetMathLibrary.BreakVector2D` (0.0 0.0)))
  (`/Engine/EditorBlueprintResources/StandardMacros.IsValid` null
    (:`Is Valid`
      (`SceneComponent.SetMobility` (`self.RootComponent`) "Movable") ; Car Actor must be Movable
      (`self.K2_AttachToComponent` (`self.SM_AutoStage_TT_CenterPlate`) "None" "SnapToTarget" "SnapToTarget" "KeepRelative") ; Set Car Actor as child to Center Plate component
      (`self.K2_AddActorLocalOffset` (`KismetMathLibrary.MakeVector` _x _y)))))

(fn `SetStageMaterials`
  (bind _wallmaterial (`self.WallMaterial`))
  (`|ExecutionSequence`
    (:`then_0`
      (`PrimitiveComponent.SetMaterial` (`self.SM_AutoStage_TT_CenterPlate`) 0 (`self.CenterPlateMaterial`)))
    (:`then_1`
      (`PrimitiveComponent.SetMaterial` (`self.SM_AutoStage_TT_OuterPlate`) 0 (`self.OuterPlateMaterial`)))
    (:`then_2`
      (`PrimitiveComponent.SetMaterial` (`self.SM_AutoStage_TT_Wall`) 0 _wallmaterial))
    (:`then_3`
      (`PrimitiveComponent.SetMaterial` (`self.SM_AutoStage_TT_Ramp`) 0 _wallmaterial))))

(fn `UserConstructionScript`
  (`StaticMeshComponent.SetStaticMesh` (`self.SM_AutoStage_TT_OuterPlate`) (select `bool` (`self.useCustomFloor`) :`false` (`BlueprintMapLibrary.Map_Find` (`self.FloorTypeMap`) (`self.FloorType`)) :`true` (`self.customFloor`))) ; Set selected outer floor mesh
  (`self.SetStageMaterials`) ; Set user selected materials
)