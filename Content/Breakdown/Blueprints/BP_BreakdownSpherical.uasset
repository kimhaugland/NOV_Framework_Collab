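; Exploded-view actor that pushes static mesh actors inside its box radially out from its center and reassembles them.
; BeginPlay gathers meshes by bounds origin, caching start location, radial direction, normalized distance and an optional delay that lets outer pieces move first.
; Breakdown toggles the target alpha, stretched to cover the longest delay.
; Tick interpolates alpha linearly or eased, offsetting each piece by distance-scaled BreakdownRadius.
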(event `self.ReceiveBeginPlay`
  (bind (_origin _boxextent) (`KismetSystemLibrary.GetComponentBounds` (`self.Box`)))
  ;[1 1 1] Find Actors to breakdown
  (bind _outactors (`GameplayStatics.GetAllActorsOfClass` "/Script/Engine.StaticMeshActor"))
  (for _array_element _outactors
    (if (!= _array_element self)
      (if (`KismetMathLibrary.IsPointInBox` (`self.GetActorBounds` _array_element true) _origin _boxextent)
        (`KismetArrayLibrary.Array_Add` (`self.ActorsToBreakdown`) _array_element))))
  (for (_array_element_2 _array_index) (`self.ActorsToBreakdown`)
    (bind _output_get (set `self.index` _array_index))
    (`KismetArrayLibrary.Array_Set` (`self.StartWorldLocation`) _output_get (`self.K2_GetActorLocation` _array_element_2) true) ; Get starting World position of individeal Actors
    (bind _returnvalue (- (`self.GetActorBounds` _array_element_2 false) (`self.animationCenter`)))
    (`KismetArrayLibrary.Array_Set` (`self.StartRadiusVector`) (`self.index`) (`KismetMathLibrary.Normal` _returnvalue) true) ; Get normalized radius vector
    (`KismetArrayLibrary.Array_Set` (`self.StartRadiusCoeff`) (`self.index`) (/ (`KismetMathLibrary.VSize` _returnvalue) (`self.BoxExtent`)) true) ; Starting position on radius vector
    (if (`self.UsePositionDelay`)
      ;[1 1 1] delay coefficient
      (`KismetArrayLibrary.Array_Add` (`self.DeltaAnimationTime`) (* (- 1.0 (`KismetMathLibrary.FClamp` (`KismetArrayLibrary.Array_Get` (`self.StartRadiusCoeff`) (`self.index`)))) (`self.AnimationDelayOveral`)))
      (else
        ;[1 1 1] delay = 0
        (`KismetArrayLibrary.Array_Add` (`self.DeltaAnimationTime`))))))

(event `self.ReceiveTick`
  (params (DeltaSeconds :type "Float (single-precision)"))
  (bind _delta (`self.delta`))
  (bind _animationalfa (`self.AnimationAlfa`))
  (bind _targetanimationalfa (`self.TargetAnimationAlfa`))
  (bind _animationspeed (`self.AnimationSpeed`))
  (set `self.delta` DeltaSeconds)
  (if (`self.AnimationStarted`)
    (if (`self.UseLinearSpeed`)
      ;[1 1 1] Linear or nonlinear speed
      (set `self.AnimationAlfa` (`KismetMathLibrary.FInterpTo_Constant` _animationalfa _targetanimationalfa _delta _animationspeed))
      (else
        (set `self.AnimationAlfa` (`KismetMathLibrary.FInterpTo` _animationalfa _targetanimationalfa _delta _animationspeed))))
    (if (!= (`self.TargetAnimationAlfa`) (`self.AnimationAlfa`))
      (`self.UpdatePositionForAnimation`)
      (elif (== (`self.TargetAnimationAlfa`) 0.0)
        (`self.UpdatePositionForAnimation`)
        (set `self.AnimationStarted` false) ; Stop animation
      ))))

(fn `AddActors`
  (params (NewItem :type "Map of Actor Object Reference to Object Object Reference (by ref)"))
  (`KismetArrayLibrary.Array_Add` (`self.ActorsToBreakdown`) null))

(fn `Breakdown`
  (if (== (`self.TargetAnimationAlfa`) 0.0)
    ;[1 1 1] Breakdown
    (bind _maxcomponent (`self.MaxOfVectorComponent` (`self.DeltaAnimationTime`)))
    (set `self.TargetAnimationAlfa` (+ _maxcomponent 1.0))
    (else
      ;[1 1 1] Compose (assembly)
      (set `self.TargetAnimationAlfa` 0.0)))
  (set `self.AnimationStarted` true))

(fn `MaxOfVectorComponent`
  (params (Array :type "Array of Float (double-precision)"))
  (returns (MaxComponent :type "Float (double-precision)"))
  (locals (localMax :type "Float (double-precision)"))
  (for _array_element Array
    (set `local.localMax` (`KismetMathLibrary.FMax` _array_element (`local.localMax`))))
  (return (`local.localMax`)))

(fn `UpdatePositionForAnimation`
  (locals (i :type Integer))
  (for (_array_element _array_index) (`self.ActorsToBreakdown`)
    (set `local.i` _array_index)
    (`self.K2_SetActorLocation` _array_element (+ (`KismetArrayLibrary.Array_Get` (`self.StartWorldLocation`) (`local.i`)) (`KismetMathLibrary.VLerp` (0.0 0.0 0.0) (* (`KismetArrayLibrary.Array_Get` (`self.StartRadiusVector`) (`local.i`)) (* (`KismetArrayLibrary.Array_Get` (`self.StartRadiusCoeff`) (`local.i`)) (`self.BreakdownRadius`))) (`KismetMathLibrary.FClamp` (- (`self.AnimationAlfa`) (`KismetArrayLibrary.Array_Get` (`self.DeltaAnimationTime`) (`local.i`))) 0.0 1.0))) false false)))

(fn `UserConstructionScript`
  (bind _boxextent (`self.BoxExtent`))
  (bind _returnvalue (* _boxextent -1.0))
  (`BoxComponent.SetBoxExtent` (`self.Box`) (`KismetMathLibrary.MakeVector` _boxextent _boxextent _boxextent) true)
  ;[1 1 1] Set position of Start-Spheres
  (`SceneComponent.K2_SetRelativeLocation` (`self.StartX`) (`KismetMathLibrary.MakeVector` _returnvalue) false false)
  (`SceneComponent.K2_SetRelativeLocation` (`self.StartY`) (`KismetMathLibrary.MakeVector` 0.0 _returnvalue) false false)
  (`SceneComponent.K2_SetRelativeLocation` (`self.StartZ`) (`KismetMathLibrary.MakeVector` 0.0 0.0 _returnvalue) false false)
  (set `self.StartStartX` (`SceneComponent.K2_GetComponentLocation` (`self.StartX`)))
  (set `self.StartStartY` (`SceneComponent.K2_GetComponentLocation` (`self.StartY`)))
  (set `self.StartStartZ` (`SceneComponent.K2_GetComponentLocation` (`self.StartZ`)))
  ;[1 1 1] Set position of End-Spheres
  (`SceneComponent.K2_SetRelativeLocation` (`self.EndX`) (`KismetMathLibrary.MakeVector` _boxextent) false false)
  (`SceneComponent.K2_SetRelativeLocation` (`self.EndY`) (`KismetMathLibrary.MakeVector` 0.0 _boxextent) false false)
  (`SceneComponent.K2_SetRelativeLocation` (`self.EndZ`) (`KismetMathLibrary.MakeVector` 0.0 0.0 _boxextent) false false)
  ;[1 1 1] Set starting vectors
  (bind _output_get (set `self.StartEndX` (`SceneComponent.K2_GetComponentLocation` (`self.EndX`))))
  (set `self.StartDirectionVectorX` (- _output_get (`self.StartStartX`)))
  (bind _output_get_2 (set `self.StartEndY` (`SceneComponent.K2_GetComponentLocation` (`self.EndY`))))
  (set `self.StartDirectionVectorY` (- _output_get_2 (`self.StartStartY`)))
  (bind _output_get_3 (set `self.StartEndZ` (`SceneComponent.K2_GetComponentLocation` (`self.EndZ`))))
  (set `self.StartDirectionVectorZ` (- _output_get_3 (`self.StartStartZ`)))
  (set `self.animationCenter` (`SceneComponent.K2_GetComponentLocation` (`self.DefaultSceneRoot`)))
  ;[1 1 1] Set billboard location
  (`SceneComponent.K2_SetRelativeLocation` (`self.Billboard`) (`KismetMathLibrary.MakeVector` 0.0 0.0 (+ (.z (`SceneComponent.RelativeLocation` (`self.EndZ`))) 30.0)) false false))