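; Exploded-view actor that spreads static mesh actors inside its box apart and reassembles them when Breakdown toggles.
; BeginPlay gathers those actors and stores each one's normalized projection onto X, Y and Z axes marked by Start/End handles.
; Tick eases one alpha and widens the handles, remapping actors along the stretched axes.
; Per-axis delays and optional position-based delays stagger motion, so outer pieces leave first and return last.
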(event `self.ReceiveBeginPlay`
  (bind _startdirectionvectory (`self.StartDirectionVectorY`))
  (bind _startdirectionvectorz (`self.StartDirectionVectorZ`))
  (bind _startdirectionvectory_2 (`self.StartDirectionVectorY`))
  (bind _startdirectionvectorz_2 (`self.StartDirectionVectorZ`))
  (bind _startdirectionvectorx (`self.StartDirectionVectorX`))
  (bind (_origin _boxextent) (`KismetSystemLibrary.GetComponentBounds` (`self.Box`)))
  ;[1 1 1] Find Actors to breakdown
  (bind _outactors (`GameplayStatics.GetAllActorsOfClass` "/Script/Engine.StaticMeshActor"))
  (for _array_element _outactors
    (if (!= _array_element self)
      (if (`KismetMathLibrary.IsPointInBox` (`self.GetActorBounds` _array_element true) _origin _boxextent)
        (`KismetArrayLibrary.Array_Add` (`self.ActorsToBreakdown`) _array_element))))
  (for (_array_element_2 _array_index) (`self.ActorsToBreakdown`)
    (bind _output_get (set `self.index` _array_index))
    (`KismetArrayLibrary.Array_Set` (`self.StartWorldLocation`) _output_get (`self.K2_GetActorLocation` _array_element_2) true) ; Get starting World position of individeal Actors
    (bind _origin_2 (`self.GetActorBounds` _array_element_2 false))
    (bind _returnvalue (- _origin_2 (`self.StartStartX`)))
    (bind _returnvalue_2 (/ (* (`KismetMathLibrary.VSize` _returnvalue) (`KismetMathLibrary.Dot_VectorVector` (`KismetMathLibrary.Normal` _returnvalue) (`KismetMathLibrary.Normal` (`self.StartDirectionVectorX`)))) (`KismetMathLibrary.VSize` (`self.StartDirectionVectorX`))))
    (bind _returnvalue_3 (- _origin_2 (`self.StartStartY`)))
    (bind _returnvalue_4 (/ (* (`KismetMathLibrary.VSize` _returnvalue_3) (`KismetMathLibrary.Dot_VectorVector` (`KismetMathLibrary.Normal` _returnvalue_3) (`KismetMathLibrary.Normal` _startdirectionvectory))) (`KismetMathLibrary.VSize` _startdirectionvectory)))
    (bind _returnvalue_5 (- _origin_2 (`self.StartStartZ`)))
    (bind _returnvalue_6 (/ (* (`KismetMathLibrary.VSize` _returnvalue_5) (`KismetMathLibrary.Dot_VectorVector` (`KismetMathLibrary.Normal` _returnvalue_5) (`KismetMathLibrary.Normal` _startdirectionvectorz))) (`KismetMathLibrary.VSize` _startdirectionvectorz)))
    (`KismetArrayLibrary.Array_Set` (`self.PositionCoeff`) (`self.index`) (`KismetMathLibrary.MakeVector` _returnvalue_2 _returnvalue_4 _returnvalue_6) true) ; Get position coefficient for all axis
    ;[1 1 1] Remember start position on X Y and Z vectors
    (`KismetArrayLibrary.Array_Set` (`self.StartPositionOnVectorWorldX`) (`self.index`) (+ (* (`KismetMathLibrary.Normal` _startdirectionvectorx) (* (`KismetMathLibrary.VSize` _startdirectionvectorx) _returnvalue_2)) (`self.StartStartX`)) true)
    (`KismetArrayLibrary.Array_Set` (`self.StartPositionOnVectorWorldY`) (`self.index`) (+ (* (`KismetMathLibrary.Normal` _startdirectionvectory_2) (* (`KismetMathLibrary.VSize` _startdirectionvectory_2) _returnvalue_4)) (`self.StartStartY`)) true)
    (`KismetArrayLibrary.Array_Set` (`self.StartPositionOnVectorWorldZ`) (`self.index`) (+ (* (`KismetMathLibrary.Normal` _startdirectionvectorz_2) (* (`KismetMathLibrary.VSize` _startdirectionvectorz_2) _returnvalue_6)) (`self.StartStartZ`)) true)
    (if (`self.UsePositionDelay`)
      ;[1 1 1] delay coefficient
      (`KismetArrayLibrary.Array_Add` (`self.DeltaAnimationTime`) (* (- (`KismetMathLibrary.MakeVector` 1.0 1.0 1.0) (* (`KismetMathLibrary.MakeVector` (`KismetMathLibrary.Abs` (.x (- (`KismetArrayLibrary.Array_Get` (`self.PositionCoeff`) (`self.index`)) 0.5))) (`KismetMathLibrary.Abs` (.y (- (`KismetArrayLibrary.Array_Get` (`self.PositionCoeff`) (`self.index`)) 0.5))) (`KismetMathLibrary.Abs` (.z (- (`KismetArrayLibrary.Array_Get` (`self.PositionCoeff`) (`self.index`)) 0.5)))) 2.0)) (`self.AnimationDelayOveral`)))
      (else
        ;[1 1 1] delay = 0
        (`KismetArrayLibrary.Array_Add` (`self.DeltaAnimationTime`) (0.0 0.0 0.0))))))

(event `self.ReceiveTick`
  (params (DeltaSeconds :type "Float (single-precision)"))
  (bind _delta (`self.delta`))
  (bind _animationalfa (`self.AnimationAlfa`))
  (bind _targetanimationalfa (`self.TargetAnimationAlfa`))
  (bind _animationspeed (`self.AnimationSpeed`))
  (set `self.delta` DeltaSeconds)
  (if (`self.AnimationStarted`)
    (if (`self.UseLinearSpeed`)
      ;[1 1 1] Linear or nonlinear speed
      (set `self.AnimationAlfa` (`KismetMathLibrary.FInterpTo_Constant` _animationalfa _targetanimationalfa _delta _animationspeed))
      (else
        (set `self.AnimationAlfa` (`KismetMathLibrary.FInterpTo` _animationalfa _targetanimationalfa _delta _animationspeed))))
    (if (!= (`self.TargetAnimationAlfa`) (`self.AnimationAlfa`))
      ;[1 1 1] Move the control spheres to the final position.
      (`SceneComponent.K2_SetWorldLocation` (`self.StartX`) (`self.TargetStartPositionX`) false false)
      (`SceneComponent.K2_SetWorldLocation` (`self.EndX`) (`self.TargetEndPositionX`) false false)
      (`SceneComponent.K2_SetWorldLocation` (`self.StartY`) (`self.TargetStartPositionY`) false false)
      (`SceneComponent.K2_SetWorldLocation` (`self.EndY`) (`self.TargetEndPositionY`) false false)
      (`SceneComponent.K2_SetWorldLocation` (`self.StartZ`) (`self.TargetStartPositionZ`) false false)
      (`SceneComponent.K2_SetWorldLocation` (`self.EndZ`) (`self.TargetEndPositionZ`) false false)
      (`self.UpdatePositionForAnimation`)
      (elif (== (`self.TargetAnimationAlfa`) 0.0)
        ;[1 1 1] Move the control spheres to the starting position.
        (`SceneComponent.K2_SetWorldLocation` (`self.StartX`) (`self.StartStartX`) false false)
        (`SceneComponent.K2_SetWorldLocation` (`self.EndX`) (`self.StartEndX`) false false)
        (`SceneComponent.K2_SetWorldLocation` (`self.StartY`) (`self.StartStartY`) false false)
        (`SceneComponent.K2_SetWorldLocation` (`self.EndY`) (`self.StartEndY`) false false)
        (`SceneComponent.K2_SetWorldLocation` (`self.StartZ`) (`self.StartStartZ`) false false)
        (`SceneComponent.K2_SetWorldLocation` (`self.EndZ`) (`self.StartEndZ`) false false)
        (set `self.AnimationStarted` false) ; Stop animation
      ))))

(fn `AddActors`
  (params (NewItem :type "Map of Actor Object Reference to Object Object Reference (by ref)"))
  (`KismetArrayLibrary.Array_Add` (`self.ActorsToBreakdown`) null))

(fn `Breakdown`
  (bind _returnvalue (* (`KismetMathLibrary.Normal` (`self.StartDirectionVectorX`)) (* (`self.BreakdownSizeX`) -0.5)))
  (bind _returnvalue_2 (* (`KismetMathLibrary.Normal` (`self.StartDirectionVectorY`)) (* (`self.BreakdownSizeY`) -0.5)))
  (bind _returnvalue_3 (* (`KismetMathLibrary.Normal` (`self.StartDirectionVectorZ`)) (* (`self.BreakdownSizeZ`) -0.5)))
  (if (== (`self.TargetAnimationAlfa`) 0.0)
    ;[1 1 1] Breakdown
    (bind _maxcomponent (`self.MaxOfVectorComponent` (`self.DeltaAnimationTime`)))
    (set `self.TargetAnimationAlfa` (+ (+ _maxcomponent 1.0) (`KismetMathLibrary.FMax` (`self.AnimationDelayX`) (`self.AnimationDelayY`) (`self.AnimationDelayZ`))))
    (set `self.AlfaHandle` 1.0)
    (else
      ;[1 1 1] Compose (assembly)
      (set `self.TargetAnimationAlfa` 0.0)))
  ;[1 1 1] Set all handles to final position (depending on Breakdown size)
  (set `self.TargetStartPositionX` (+ (`self.StartStartX`) _returnvalue))
  (set `self.TargetEndPositionX` (- (`self.StartEndX`) _returnvalue))
  (set `self.TargetStartPositionY` (+ (`self.StartStartY`) _returnvalue_2))
  (set `self.TargetEndPositionY` (- (`self.StartEndY`) _returnvalue_2))
  (set `self.TargetStartPositionZ` (+ (`self.StartStartZ`) _returnvalue_3))
  (set `self.TargetEndPositionZ` (- (`self.StartEndZ`) _returnvalue_3))
  (set `self.AnimationStarted` true))

(fn `MaxOfVectorComponent`
  (params (Array :type "Array of Vector Structure"))
  (returns (MaxComponent :type "Float (double-precision)"))
  (locals (localMax :type "Float (double-precision)"))
  (for _array_element Array
    (set `local.localMax` (`KismetMathLibrary.FMax` (.x _array_element) (.y _array_element) (.z _array_element) (`local.localMax`))))
  (return (`local.localMax`)))

(fn `UpdatePositionForAnimation`
  (locals (i :type Integer) (`Start X Current` :type "Vector Structure") (`X Current Length` :type "Float (double-precision)") (`X Current Direction` :type "Vector Structure") (`Start Y Current` :type "Vector Structure") (`Y Current Length` :type "Float (double-precision)") (`Y Current Direction` :type "Vector Structure") (`Start Z Current` :type "Vector Structure") (`Z Current Length` :type "Float (double-precision)") (`Z Current Direction` :type "Vector Structure"))
  (bind _animationalfa (`self.AnimationAlfa`))
  (bind _returnvalue (- (`SceneComponent.K2_GetComponentLocation` (`self.EndX`)) (`local.Start X Current`)))
  (bind _returnvalue_2 (- (`SceneComponent.K2_GetComponentLocation` (`self.EndY`)) (`local.Start Y Current`)))
  (bind _returnvalue_3 (- (`SceneComponent.K2_GetComponentLocation` (`self.EndZ`)) (`local.Start Z Current`)))
  ;[1 1 1] Precalculate positions
  (set `local.Start X Current` (`SceneComponent.K2_GetComponentLocation` (`self.StartX`)))
  (set `local.X Current Length` (`KismetMathLibrary.VSize` _returnvalue))
  (set `local.X Current Direction` (`KismetMathLibrary.Normal` _returnvalue))
  (set `local.Start Y Current` (`SceneComponent.K2_GetComponentLocation` (`self.StartY`)))
  (set `local.Y Current Length` (`KismetMathLibrary.VSize` _returnvalue_2))
  (set `local.Y Current Direction` (`KismetMathLibrary.Normal` _returnvalue_2))
  (set `local.Start Z Current` (`SceneComponent.K2_GetComponentLocation` (`self.StartZ`)))
  (set `local.Z Current Length` (`KismetMathLibrary.VSize` _returnvalue_3))
  (set `local.Z Current Direction` (`KismetMathLibrary.Normal` _returnvalue_3))
  (for (_array_element _array_index) (`self.ActorsToBreakdown`)
    (set `local.i` _array_index)
    (`self.K2_SetActorLocation` _array_element (+ (`KismetArrayLibrary.Array_Get` (`self.StartWorldLocation`) (`local.i`)) (+ (`KismetMathLibrary.VLerp` (0.0 0.0 0.0) (- (+ (* (`local.X Current Direction`) (* (.x (`KismetArrayLibrary.Array_Get` (`self.PositionCoeff`) (`local.i`))) (`local.X Current Length`))) (`local.Start X Current`)) (`KismetArrayLibrary.Array_Get` (`self.StartPositionOnVectorWorldX`) (`local.i`))) (`KismetMathLibrary.FClamp` (- (- _animationalfa (.x (`KismetArrayLibrary.Array_Get` (`self.DeltaAnimationTime`) (`local.i`)))) (`self.AnimationDelayX`)) 0.0 1.0)) (`KismetMathLibrary.VLerp` (0.0 0.0 0.0) (- (+ (* (`local.Y Current Direction`) (* (.y (`KismetArrayLibrary.Array_Get` (`self.PositionCoeff`) (`local.i`))) (`local.Y Current Length`))) (`local.Start Y Current`)) (`KismetArrayLibrary.Array_Get` (`self.StartPositionOnVectorWorldY`) (`local.i`))) (`KismetMathLibrary.FClamp` (- (- _animationalfa (.y (`KismetArrayLibrary.Array_Get` (`self.DeltaAnimationTime`) (`local.i`)))) (`self.AnimationDelayY`)) 0.0 1.0)) (`KismetMathLibrary.VLerp` (0.0 0.0 0.0) (- (+ (* (`local.Z Current Direction`) (* (.z (`KismetArrayLibrary.Array_Get` (`self.PositionCoeff`) (`local.i`))) (`local.Z Current Length`))) (`local.Start Z Current`)) (`KismetArrayLibrary.Array_Get` (`self.StartPositionOnVectorWorldZ`) (`local.i`))) (`KismetMathLibrary.FClamp` (- (- _animationalfa (.z (`KismetArrayLibrary.Array_Get` (`self.DeltaAnimationTime`) (`local.i`)))) (`self.AnimationDelayZ`)) 0.0 1.0)))) false false)))

(fn `UserConstructionScript`
  (bind _boxextent (`self.BoxExtent`))
  (bind _returnvalue (* _boxextent -1.0))
  (`BoxComponent.SetBoxExtent` (`self.Box`) (`KismetMathLibrary.MakeVector` _boxextent _boxextent _boxextent) true)
  ;[1 1 1] Set position of Start-Spheres
  (`SceneComponent.K2_SetRelativeLocation` (`self.StartX`) (`KismetMathLibrary.MakeVector` _returnvalue) false false)
  (`SceneComponent.K2_SetRelativeLocation` (`self.StartY`) (`KismetMathLibrary.MakeVector` 0.0 _returnvalue) false false)
  (`SceneComponent.K2_SetRelativeLocation` (`self.StartZ`) (`KismetMathLibrary.MakeVector` 0.0 0.0 _returnvalue) false false)
  (set `self.StartStartX` (`SceneComponent.K2_GetComponentLocation` (`self.StartX`)))
  (set `self.StartStartY` (`SceneComponent.K2_GetComponentLocation` (`self.StartY`)))
  (set `self.StartStartZ` (`SceneComponent.K2_GetComponentLocation` (`self.StartZ`)))
  ;[1 1 1] Set position of End-Spheres
  (`SceneComponent.K2_SetRelativeLocation` (`self.EndX`) (`KismetMathLibrary.MakeVector` _boxextent) false false)
  (`SceneComponent.K2_SetRelativeLocation` (`self.EndY`) (`KismetMathLibrary.MakeVector` 0.0 _boxextent) false false)
  (`SceneComponent.K2_SetRelativeLocation` (`self.EndZ`) (`KismetMathLibrary.MakeVector` 0.0 0.0 _boxextent) false false)
  ;[1 1 1] Set starting vectors
  (bind _output_get (set `self.StartEndX` (`SceneComponent.K2_GetComponentLocation` (`self.EndX`))))
  (set `self.StartDirectionVectorX` (- _output_get (`self.StartStartX`)))
  (bind _output_get_2 (set `self.StartEndY` (`SceneComponent.K2_GetComponentLocation` (`self.EndY`))))
  (set `self.StartDirectionVectorY` (- _output_get_2 (`self.StartStartY`)))
  (bind _output_get_3 (set `self.StartEndZ` (`SceneComponent.K2_GetComponentLocation` (`self.EndZ`))))
  (set `self.StartDirectionVectorZ` (- _output_get_3 (`self.StartStartZ`)))
  (set `self.animationCenter` (* (+ (`self.StartStartX`) (`self.StartEndX`)) 0.5))
  ;[1 1 1] Set billboard location
  (`SceneComponent.K2_SetRelativeLocation` (`self.Billboard`) (`KismetMathLibrary.MakeVector` 0.0 0.0 (+ (.z (`SceneComponent.RelativeLocation` (`self.EndZ`))) 30.0)) false false))