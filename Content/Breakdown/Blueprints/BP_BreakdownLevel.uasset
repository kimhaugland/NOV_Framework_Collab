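; Level actor that animates mesh actors dropping into place to assemble the level, or rising away to disassemble it.
; Breakdown and BreakdownInverted gather movable static and skeletal mesh actors; only Breakdown honors an optional bounding box.
; Each actor's delay, weighted by index, position and size, doubles as its Z offset.
; Tick shifts offsets by AnimationSpeed per frame, without delta-time scaling, producing a staggered cascade.
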(event `self.ReceiveTick`
  (params (DeltaSeconds :type "Float (single-precision)"))
  (bind _item (`KismetArrayLibrary.Array_Get` (`self.AnimationDelayArray`) (`self.index`)))
  (if (`self.animation active`)
    ;[1 1 1] Forward Cycle (level assembly)
    (set `self.animation active` false) ; Set this flag to false. If flag is still false by the end of the loop - animation is over
    (for (_array_element _array_index) (`self.ActorsArray`)
      (set `self.index` _array_index)
      (if (> (`KismetArrayLibrary.Array_Get` (`self.AnimationDelayArray`) (`self.index`)) 0.0)
        ;;[1 1 1] Set Actor location and Delay
        (`self.K2_SetActorLocation` _array_element (`KismetMathLibrary.MakeVector` (.x (`KismetArrayLibrary.Array_Get` (`self.InitialZArray`) (`self.index`))) (.y (`KismetArrayLibrary.Array_Get` (`self.InitialZArray`) (`self.index`))) (+ (.z (`KismetArrayLibrary.Array_Get` (`self.InitialZArray`) (`self.index`))) _item)) false false)
        (`KismetArrayLibrary.Array_Set` (`self.AnimationDelayArray`) (`self.index`) (- _item (`self.AnimationSpeed`)))
        (set `self.animation active` true) ; Continue animation on the next frame
        (else
          ;;[1 1 1] Finalize object animation
          (`KismetArrayLibrary.Array_Set` (`self.AnimationDelayArray`) (`self.index`))
          (`self.K2_SetActorLocation` _array_element (`KismetArrayLibrary.Array_Get` (`self.InitialZArray`) (`self.index`)) false false))))
    (else
      ;[1 1 1] Backward Cycle (level disassembly)
      (if (`self.animation active inverted`)
        (for (_array_element_2 _array_index_2) (`self.ActorsArray`)
          (set `self.index` _array_index_2)
          (if (> (`self.MaxAnimationDelay`) 0.0)
            ;;[1 1 1] Set Actor location and Delay
            (if (> (- (`KismetArrayLibrary.Array_Get` (`self.AnimationDelayArray`) (`self.index`)) (`self.MaxAnimationDelay`)) 0.0)
              (`self.K2_SetActorLocation` _array_element_2 (`KismetMathLibrary.MakeVector` (.x (`KismetArrayLibrary.Array_Get` (`self.InitialZArray`) (`self.index`))) (.y (`KismetArrayLibrary.Array_Get` (`self.InitialZArray`) (`self.index`))) (+ (.z (`KismetArrayLibrary.Array_Get` (`self.InitialZArray`) (`self.index`))) (- (`KismetArrayLibrary.Array_Get` (`self.AnimationDelayArray`) (`self.index`)) (`self.MaxAnimationDelay`)))) false false))
            (else
              ;;[1 1 1] Finalize object animation
              (set `self.animation active inverted` false))))
        (set `self.MaxAnimationDelay` (- (`self.MaxAnimationDelay`) (`self.AnimationSpeed`)))))))

(fn `Breakdown`
  (params (`Do not recalculate oblect position` :type Boolean))
  (locals (`Custom Box Origin` :type "Vector Structure") (`Custom Box Extent` :type "Vector Structure"))
  (bind (_origin _boxextent) (`self.GetActorBounds` (`self.CustomBoundBox`) false))
  (bind (_origin_2 _boxextent_2) (`self.GetActorBounds` (`self.CustomBoundBox`) false))
  (if (not (`self.animation active`))
    (if (not `Do not recalculate oblect position`)
      (`|ExecutionSequence`
        (:`then_0`
          ;[1 1 1] Add StaticMeshActors - movable only
          (if (`self.Animate StaticMeshActors`)
            (if (!= (`self.CustomBoundBox`) null)
              (set `local.Custom Box Origin` _origin)
              (set `local.Custom Box Extent` _boxextent))
            (bind _outactors (`GameplayStatics.GetAllActorsOfClass` "/Script/Engine.StaticMeshActor"))
            (for _array_element _outactors
              (bind _asstatic_mesh_actor (cast `StaticMeshActor` _array_element))
              (if (== (`self.CustomBoundBox`) null)
                (bind _staticmeshcomponent (`StaticMeshActor.StaticMeshComponent` _asstatic_mesh_actor))
                (if (`|EnumEquality` (`SceneComponent.Mobility` _staticmeshcomponent) "Movable") :!label _label
                  (if (`self.TurnOffPhysicsSimulation`)
                    (`PrimitiveComponent.SetSimulatePhysics` _staticmeshcomponent false) ; Turn off physic simulation
                  )
                  (`KismetArrayLibrary.Array_Add` (`self.ActorsArray`) _asstatic_mesh_actor)
                  (bind _returnvalue (`self.K2_GetActorLocation` _asstatic_mesh_actor))
                  (`KismetArrayLibrary.Array_Add` (`self.InitialZArray`) _returnvalue)
                  ;;[1 1 1] Delays should be only positive so we need to get minimum positions
                  (set `self.MinXLocation` (`KismetMathLibrary.FMin` (.x _returnvalue) (`self.MinXLocation`)))
                  (set `self.MinYLocation` (`KismetMathLibrary.FMin` (.y _returnvalue) (`self.MinYLocation`)))
                  (set `self.MinZLocation` (`KismetMathLibrary.FMin` (.z _returnvalue) (`self.MinZLocation`))))
                (elif (`KismetMathLibrary.IsPointInBox` (`self.GetActorBounds` _asstatic_mesh_actor true) (`local.Custom Box Origin`) (`local.Custom Box Extent`))
                  (goto _label))))))
        (:`then_1`
          ;[1 1 1] Add SkeletalMeshActors
          (if (`self.Animate SkeletalMeshActors`)
            (if (!= (`self.CustomBoundBox`) null)
              (set `local.Custom Box Origin` _origin_2)
              (set `local.Custom Box Extent` _boxextent_2))
            (bind _outactors_2 (`GameplayStatics.GetAllActorsOfClass` "/Script/Engine.SkeletalMeshActor"))
            (for _array_element_2 _outactors_2
              (if (== (`self.CustomBoundBox`) null)
                (`KismetArrayLibrary.Array_Add` (`self.ActorsArray`) _array_element_2 :!label _label_2)
                (bind _returnvalue_2 (`self.K2_GetActorLocation` _array_element_2))
                (`KismetArrayLibrary.Array_Add` (`self.InitialZArray`) _returnvalue_2)
                ;;[1 1 1] Delays should be only positive so we need to get minimum positions
                (set `self.MinXLocation` (`KismetMathLibrary.FMin` (.x _returnvalue_2) (`self.MinXLocation`)))
                (set `self.MinYLocation` (`KismetMathLibrary.FMin` (.y _returnvalue_2) (`self.MinYLocation`)))
                (set `self.MinZLocation` (`KismetMathLibrary.FMin` (.z _returnvalue_2) (`self.MinZLocation`)))
                (elif (`KismetMathLibrary.IsPointInBox` (`self.GetActorBounds` true) (`local.Custom Box Origin`) (`local.Custom Box Extent`))
                  (goto _label_2))))))
        (:`then_2`
          ;[1 1 1] Calculate animation delay for all collected Actors
          (for (_array_element_3 _array_index) (`self.ActorsArray`)
            (bind (_origin_3 _boxextent_3) (`self.GetActorBounds` _array_element_3 false))
            (`KismetArrayLibrary.Array_Add` (`self.AnimationDelayArray`) (+ (* _array_index (`self.DelayIndex`)) (* (- (.x _origin_3) (`self.MinXLocation`)) (`self.DelayLocationX`)) (* (- (.y _origin_3) (`self.MinYLocation`)) (`self.DelayLocationY`)) (* (- (.z _origin_3) (`self.MinZLocation`)) (`self.DelayLocationZ`)) (* (`KismetMathLibrary.VSize` _boxextent_3) (`self.DelaySize`)) (`self.StaticDelay`)))))
        (:`then_3`
          ;[1 1 1] Start animation
          (set `self.animation active` true :!label _label_3)))
      (else
        (goto _label_3)))))

(fn `BreakdownInverted`
  (if (not (`self.animation active`))
    (`|ExecutionSequence`
      (:`then_0`
        ;[1 1 1] Add StaticMeshActors - movable only
        (if (`self.Animate StaticMeshActors`)
          (bind _outactors (`GameplayStatics.GetAllActorsOfClass` "/Script/Engine.StaticMeshActor"))
          (for _array_element _outactors
            (bind _asstatic_mesh_actor (cast `StaticMeshActor` _array_element))
            (bind _staticmeshcomponent (`StaticMeshActor.StaticMeshComponent` _asstatic_mesh_actor))
            (if (`|EnumEquality` (`SceneComponent.Mobility` _staticmeshcomponent) "Movable")
              (if (`self.TurnOffPhysicsSimulation`)
                (`PrimitiveComponent.SetSimulatePhysics` _staticmeshcomponent false) ; Turn off physic simulation
              )
              (`KismetArrayLibrary.Array_Add` (`self.ActorsArray`) _asstatic_mesh_actor)
              (bind _returnvalue (`self.K2_GetActorLocation` _asstatic_mesh_actor))
              (`KismetArrayLibrary.Array_Add` (`self.InitialZArray`) _returnvalue)
              ;;[1 1 1] Delays should be only positive so we need to get minimum positions
              (set `self.MinXLocation` (`KismetMathLibrary.FMin` (.x _returnvalue) (`self.MinXLocation`)))
              (set `self.MinYLocation` (`KismetMathLibrary.FMin` (.y _returnvalue) (`self.MinYLocation`)))
              (set `self.MinZLocation` (`KismetMathLibrary.FMin` (.z _returnvalue) (`self.MinZLocation`)))))))
      (:`then_1`
        ;[1 1 1] Add SkeletalMeshActors
        (if (`self.Animate SkeletalMeshActors`)
          (bind _outactors_2 (`GameplayStatics.GetAllActorsOfClass` "/Script/Engine.SkeletalMeshActor"))
          (for _array_element_2 _outactors_2
            (`KismetArrayLibrary.Array_Add` (`self.ActorsArray`) _array_element_2)
            (bind _returnvalue_2 (`self.K2_GetActorLocation` _array_element_2))
            (`KismetArrayLibrary.Array_Add` (`self.InitialZArray`) _returnvalue_2)
            ;;[1 1 1] Delays should be only positive so we need to get minimum positions
            (set `self.MinXLocation` (`KismetMathLibrary.FMin` (.x _returnvalue_2) (`self.MinXLocation`)))
            (set `self.MinYLocation` (`KismetMathLibrary.FMin` (.y _returnvalue_2) (`self.MinYLocation`)))
            (set `self.MinZLocation` (`KismetMathLibrary.FMin` (.z _returnvalue_2) (`self.MinZLocation`))))))
      (:`then_2`
        ;[1 1 1] Calculate animation delay for all collected Actors
        (for (_array_element_3 _array_index) (`self.ActorsArray`)
          (bind (_origin _boxextent) (`self.GetActorBounds` _array_element_3 false))
          (`KismetArrayLibrary.Array_Add` (`self.AnimationDelayArray`) (+ (* _array_index (`self.DelayIndex`)) (* (- (.x _origin) (`self.MinXLocation`)) (`self.DelayLocationX`)) (* (- (.y _origin) (`self.MinYLocation`)) (`self.DelayLocationY`)) (* (- (.z _origin) (`self.MinZLocation`)) (`self.DelayLocationZ`)) (* (`KismetMathLibrary.VSize` _boxextent) (`self.DelaySize`)) (`self.StaticDelay`))))
        (set `self.MaxAnimationDelay` (`.MaxValue` (`KismetMathLibrary.MaxOfFloatArray` (`self.AnimationDelayArray`)))))
      (:`then_3`
        ;[1 1 1] Start animation
        (set `self.animation active inverted` true)))))

(fn `UserConstructionScript`)